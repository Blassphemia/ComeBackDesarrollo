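; BP_GameMode manages a single "save1" save slot for SAM's position and level restarts.
; An initial custom event loads the slot or creates it from Location_SAVEGAME, but the code restoring SAM's saved transform is disconnected.
; Savegame stores the player transform and sets a saved-location flag, which ChangeLevel clears.
; LoadGame restarts the level by console command, while RestartLevel deletes the slot first.
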(event `CustomEvent`
  (bind _returnvalue (`GameplayStatics.DoesSaveGameExist` "save1"))
  (if _returnvalue
    (bind _returnvalue_2 (`GameplayStatics.LoadGameFromSlot` "save1"))
    (bind _assam_save (cast `/Game/BP_SAM_save` _returnvalue_2))
    (if true
      _)
    (else
      ;[1 1 1] Guardado del juego
      (bind _returnvalue_3 (`GameplayStatics.CreateSaveGameObject` "/Game/Come_Back/Mi_Personaje/Mecanicas_Del_Jugador/CheckPoints/Location_SAVEGAME.Location_SAVEGAME_C"))
      (`GameplayStatics.SaveGameToSlot` _returnvalue_3 "save1"))))

(event `Save game`
  ;[1 1 1] Save Game
  (bind _returnvalue (`GameplayStatics.LoadGameFromSlot` "save1"))
  (bind _assam_save (cast `/Game/BP_SAM_save` _returnvalue))
  (set `/Game/BP_SAM_save.SAM_Transform` (`self.GetTransform` (cast `/Game/Come_Back/Mi_Personaje/SAM` (`GameplayStatics.GetPlayerCharacter` 0) :!pure true)) _assam_save)
  (set `/Game/BP_SAM_save.UserSavedLocation` true _assam_save)
  (`GameplayStatics.SaveGameToSlot` _assam_save "save1"))

(event `Load Game`
  ;[1 1 1] Cargar nivel
  (`KismetSystemLibrary.ExecuteConsoleCommand` "RestartLevel" null))

(event `RestartLevel`
  ;[1 1 1] Eliminar guardado + Restart
  (`GameplayStatics.DeleteGameInSlot` "save1")
  (`KismetSystemLibrary.ExecuteConsoleCommand` "RestartLevel" null))

(event `Change Level`
  ;[1 1 1] Cambio de Niveles
  (bind _returnvalue (`GameplayStatics.LoadGameFromSlot` "save1"))
  (bind _assam_save (cast `/Game/BP_SAM_save` _returnvalue))
  (set `/Game/BP_SAM_save.UserSavedLocation` false _assam_save)
  (`GameplayStatics.SaveGameToSlot` _assam_save "save1"))

(fn `UserConstructionScript`)