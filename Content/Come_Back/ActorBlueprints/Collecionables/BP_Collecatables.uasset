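; BP_Collecatables is a collectible actor that reacts when the SAM character overlaps its Collision component.
; The overlap plays a collection montage on the player's mesh and starts the Atraccion timeline alongside it.
; Each update moves Nave to a fixed offset from SAM, as zero-alpha lerps cancel the timeline's Distance blend.
; The actor destroys itself three seconds after the timeline finishes.
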(event `self.Collision.OnComponentBeginOverlap`
  (params (OverlappedComponent :type "PrimitiveComponent Object Reference") (OtherActor :type "Actor Object Reference") (OtherComp :type "PrimitiveComponent Object Reference") (OtherBodyIndex :type Integer) (bFromSweep :type Boolean) (SweepResult :type "HitResult Structure (by ref)"))
  ;[0 0 0] Funcion
  (bind _assam (cast `/Game/Come_Back/Mi_Personaje/SAM` OtherActor))
  (`|PlayMontage` (`Character.Mesh` (cast `/Game/Come_Back/Mi_Personaje/SAM` (`GameplayStatics.GetPlayerCharacter` 0) :!pure true)) "/Game/Come_Back/Mi_Personaje/Animaciones/Coleccionables_Sam_Montage.Coleccionables_Sam_Montage"
    (:`then`
      (bind (_direction _distance) (`Timeline|Atraccion` :!via `PlayFromStart`)
        (:`Update`
          (bind _returnvalue (`self.K2_GetActorLocation` _assam))
          (`SceneComponent.K2_SetWorldLocation` (`self.Nave`) (`KismetMathLibrary.VLerp` (`KismetMathLibrary.VLerp` (+ _returnvalue (0.0 50.0 -100.0)) (0.0 25.0 0.0)) (`KismetMathLibrary.VLerp` (`SceneComponent.K2_GetComponentLocation` (`self.Nave`)) _returnvalue _distance)) false false))
        (:`Finished`
          (`KismetSystemLibrary.Delay` 3.0)
          (`self.K2_DestroyActor`))))))

(fn `UserConstructionScript`)