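; JumpScare_BP is a one-shot tentacle jump scare triggered when something enters its box volume.
; The skeletal mesh starts hidden with collision disabled.
; The first overlap, gated by a DoOnce with no actor filter, waits briefly and starts the tentacle animation montage.
; After another short delay it plays the scare sound at the mesh, reveals it and enables query and physics collision.
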(event `self.ReceiveBeginPlay`
  (bind _skeletalmesh (`self.SkeletalMesh`))
  (`SceneComponent.SetHiddenInGame` _skeletalmesh true false)
  (`PrimitiveComponent.SetCollisionEnabled` _skeletalmesh "NoCollision"))

(event `self.Box.OnComponentBeginOverlap`
  (params (OverlappedComponent :type "PrimitiveComponent Object Reference") (OtherActor :type "Actor Object Reference") (OtherComp :type "PrimitiveComponent Object Reference") (OtherBodyIndex :type Integer) (bFromSweep :type Boolean) (SweepResult :type "HitResult Structure (by ref)"))
  (bind _skeletalmesh (`self.SkeletalMesh`))
  (`/Engine/EditorBlueprintResources/StandardMacros.DoOnce` false
    (:`Completed`
      (`KismetSystemLibrary.Delay` 0.2)
      (`SkeletalMeshComponent.PlayAnimation` _skeletalmesh "/Game/Come_Back/ActorBlueprints/Mounstro/Modelo/Tentaculo_Animado_Final_Anim_Montage.Tentaculo_Animado_Final_Anim_Montage" false)
      (`KismetSystemLibrary.Delay` 0.2)
      (`GameplayStatics.PlaySoundAtLocation` "/Game/Come_Back/Sonidos/JumpScare_.JumpScare_" (`SceneComponent.K2_GetComponentLocation` _skeletalmesh) (struct) 1.0 1.0 0.0 null null null null)
      (`SceneComponent.SetHiddenInGame` _skeletalmesh false false)
      (`PrimitiveComponent.SetCollisionEnabled` _skeletalmesh "QueryAndPhysics"))))

(fn `UserConstructionScript`)