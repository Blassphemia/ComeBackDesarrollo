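; BP_Basura is a physics object that SAM pushes until it falls, forming a bridge.
; While the push input is active, Tick enables physics on Mover; moving on Y inside the Empujar trigger slows SAM, widens the capsule and sets EstaEmpujando.
; When Box1 ends overlap with anything but FloorActor, it frees the constraint's Z and twist limits, adds mass, and disables player input during the fall.
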(event `self.ReceiveBeginPlay`
  (bind _assam (cast `/Game/Come_Back/Mi_Personaje/SAM` (`GameplayStatics.GetPlayerCharacter` 0)))
  (set `self.PlayerRef` _assam))

(event `self.empujar.OnComponentBeginOverlap`
  (params (OverlappedComponent :type "PrimitiveComponent Object Reference") (OtherActor :type "Actor Object Reference") (OtherComp :type "PrimitiveComponent Object Reference") (OtherBodyIndex :type Integer) (bFromSweep :type Boolean) (SweepResult :type "HitResult Structure (by ref)"))
  ;[1 1 1] Cuando empuje, el radio de la capsula de sam se reduce a 55
  (if (== OtherActor (`self.PlayerRef`))
    (set `self.Tick` true)
    (`CapsuleComponent.SetCapsuleRadius` (`Character.CapsuleComponent` (`self.PlayerRef`)) 55.0 false)
    (else
      (set `self.Tick` false))))

(event `self.empujar.OnComponentEndOverlap`
  (params (OverlappedComponent :type "PrimitiveComponent Object Reference") (OtherActor :type "Actor Object Reference") (OtherComp :type "PrimitiveComponent Object Reference") (OtherBodyIndex :type Integer))
  (bind _playerref (`self.PlayerRef`))
  ;[1 1 1] Cuando Sam salga del trigger, su velocidad será normal y su radio disminuirá al original
  (if (== OtherActor (`self.PlayerRef`))
    (set `self.Tick` false)
    (set `CharacterMovementComponent.MaxWalkSpeed` 300.0 (`Character.CharacterMovement` _playerref))
    (set `/Game/Come_Back/Mi_Personaje/SAM.EstaEmpujando` false _playerref)
    (`CapsuleComponent.SetCapsuleRadius` (`Character.CapsuleComponent` (`self.PlayerRef`)) 40.4 false)))

(event `self.ReceiveTick`
  (params (DeltaSeconds :type "Float (single-precision)"))
  (bind _playerref (`self.PlayerRef`))
  (bind _mover (`self.Mover`))
  (bind _charactermovement (`Character.CharacterMovement` _playerref))
  ;[1 1 1] Activación/Desactivación de físicas
  (if (`/Game/Come_Back/Mi_Personaje/SAM.Empujar` (`self.PlayerRef`))
    (`PrimitiveComponent.SetSimulatePhysics` _mover true)
    ;[1 1 1] cambio de velocidad de Sam al empujar y dejar de empujar
    (if (`self.Tick`)
      (if (!= (.y (`MovementComponent.Velocity` (`Character.CharacterMovement` (`self.PlayerRef`)))) 0.0)
        (set `/Game/Come_Back/Mi_Personaje/SAM.EstaEmpujando` true _playerref)
        (set `CharacterMovementComponent.MaxWalkSpeed` 150.0 _charactermovement)
        ;[1 1 1] Cambio del radio de sam al empujar y dejar de empujar
        (`KismetSystemLibrary.Delay` 0.1)
        (`CapsuleComponent.SetCapsuleRadius` (`Character.CapsuleComponent` (`self.PlayerRef`)) 55.0 true)
        (else
          (set `/Game/Come_Back/Mi_Personaje/SAM.EstaEmpujando` false _playerref :!label _label)
          (set `CharacterMovementComponent.MaxWalkSpeed` 300.0 _charactermovement)
          (`CapsuleComponent.SetCapsuleRadius` (`Character.CapsuleComponent` (`self.PlayerRef`)) 40.4 false))))
    (elif (`self.Cayendo`)
      (`PrimitiveComponent.SetSimulatePhysics` _mover true)
      (else
        (`PrimitiveComponent.SetSimulatePhysics` _mover false)
        (goto _label)))))

(event `self.Box1.OnComponentEndOverlap`
  (params (OverlappedComponent :type "PrimitiveComponent Object Reference") (OtherActor :type "Actor Object Reference") (OtherComp :type "PrimitiveComponent Object Reference") (OtherBodyIndex :type Integer))
  (bind _physicsconstraint (`self.PhysicsConstraint`))
  ;[1 1 1] Simula físicas y colisiones para que caiga el puente después del end overlap
  (`self.DisableInput` (`GameplayStatics.GetPlayerCharacter` 0) null)
  (if (not (== OtherComp (`self.FloorActor`)))
    (set `self.Cayendo` true)
    (`PrimitiveComponent.SetAllMassScale` (`self.Mover`) 2500.0)
    (`PhysicsConstraintComponent.SetLinearZLimit` _physicsconstraint "LCM_Free" 0.0)
    (`PhysicsConstraintComponent.SetAngularTwistLimit` _physicsconstraint "ACM_Free" 0.0)
    (`PrimitiveComponent.SetSimulatePhysics` (`self.Mover`) true)
    (`KismetSystemLibrary.Delay` 2.0)
    (`PrimitiveComponent.SetCollisionEnabled` (`self.Box1`) "NoCollision")
    (set `self.Tick` false)
    (`SceneComponent.K2_SetWorldLocation` (`self.empujar`) (0.0 -146.655457 -95.549492) false false)
    (`self.EnableInput` (`GameplayStatics.GetPlayerCharacter` 0) null)))

(fn `UserConstructionScript`)