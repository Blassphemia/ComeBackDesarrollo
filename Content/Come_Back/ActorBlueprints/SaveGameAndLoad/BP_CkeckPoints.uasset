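; One-shot checkpoint actor that saves the game when anything overlaps its Save component, then destroys itself.
; On overlap it loads SaveGameData1, adds itself to CheckPointUsed if absent, and writes that object back with an empty slot name.
; It then calls SaveGame on GameMode_Mechanics_Gamplepay_SAM.
; On BeginPlay it destroys itself if the loaded save already lists it as used.
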(event `self.Save.OnComponentBeginOverlap`
  (params (OverlappedComponent :type "PrimitiveComponent Object Reference") (OtherActor :type "Actor Object Reference") (OtherComp :type "PrimitiveComponent Object Reference") (OtherBodyIndex :type Integer) (bFromSweep :type Boolean) (SweepResult :type "HitResult Structure (by ref)"))
  (bind _returnvalue (`GameplayStatics.LoadGameFromSlot` "SaveGameData1"))
  (bind _asbp_save_game (cast `/Game/Come_Back/ActorBlueprints/SaveGameAndLoad/BP-SaveGame` _returnvalue))
  (if (not (`KismetArrayLibrary.Array_Contains` (`/Game/Come_Back/ActorBlueprints/SaveGameAndLoad/BP-SaveGame.CheckPointUsed` _asbp_save_game) self))
    (`KismetArrayLibrary.Array_Add` (`/Game/Come_Back/ActorBlueprints/SaveGameAndLoad/BP-SaveGame.CheckPointUsed` _asbp_save_game) self)
    (`GameplayStatics.SaveGameToSlot` _asbp_save_game)
    (bind _asgame_mode_mechanics_gamplepay_sam (cast `/Game/Come_Back/Mi_Personaje/Mecanicas_Del_Jugador/GameMode_Mechanics_Gamplepay_SAM` (`GameplayStatics.GetGameMode`)))
    (`/Game/Come_Back/Mi_Personaje/Mecanicas_Del_Jugador/GameMode_Mechanics_Gamplepay_SAM.SaveGame` _asgame_mode_mechanics_gamplepay_sam)
    (`self.K2_DestroyActor`)))

(event `self.ReceiveBeginPlay`
  (bind _returnvalue (`GameplayStatics.LoadGameFromSlot` "SaveGameData1"))
  (bind _asbp_save_game (cast `/Game/Come_Back/ActorBlueprints/SaveGameAndLoad/BP-SaveGame` _returnvalue))
  (if (`KismetArrayLibrary.Array_Contains` (`/Game/Come_Back/ActorBlueprints/SaveGameAndLoad/BP-SaveGame.CheckPointUsed` _asbp_save_game) self)
    (`self.K2_DestroyActor`)))

(fn `UserConstructionScript`)