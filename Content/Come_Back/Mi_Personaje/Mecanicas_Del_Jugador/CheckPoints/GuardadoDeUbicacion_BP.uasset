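; GuardadoDeUbicacion_BP is a checkpoint actor that saves a location when the SAM character overlaps its Checkpoint component.
; It loads the existing Location_SAVEGAME from the checkpoint slot, or creates one if none exists.
; It stores the actor's own location, raised above its origin with rotation and scale reset, then writes the slot and prints a debug confirmation.
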(event `self.Checkpoint.OnComponentBeginOverlap`
  (params (OverlappedComponent :type "PrimitiveComponent Object Reference") (OtherActor :type "Actor Object Reference") (OtherComp :type "PrimitiveComponent Object Reference") (OtherBodyIndex :type Integer) (bFromSweep :type Boolean) (SweepResult :type "HitResult Structure (by ref)"))
  (bind _returnvalue_location (`KismetMathLibrary.BreakTransform` (`self.GetTransform`)))
  (cast `/Game/Come_Back/Mi_Personaje/SAM` OtherActor)
  (bind _returnvalue (`GameplayStatics.DoesSaveGameExist` (`self.CheckpontSave`)))
  (if _returnvalue
    (bind _returnvalue_2 (`GameplayStatics.LoadGameFromSlot` (`self.CheckpontSave`)))
    (bind _aslocation_savegame (cast `/Game/Come_Back/Mi_Personaje/Mecanicas_Del_Jugador/CheckPoints/Location_SAVEGAME` _returnvalue_2))
    (set `self.SaveGameReference` _aslocation_savegame)
    (else
      (bind _returnvalue_3 (`GameplayStatics.CreateSaveGameObject` "/Game/Come_Back/Mi_Personaje/Mecanicas_Del_Jugador/CheckPoints/Location_SAVEGAME.Location_SAVEGAME_C"))
      (set `self.SaveGameReference` _returnvalue_3)))
  (bind _output_get (set `/Game/Come_Back/Mi_Personaje/Mecanicas_Del_Jugador/CheckPoints/Location_SAVEGAME.Checkpont` (`KismetMathLibrary.MakeTransform` (+ _returnvalue_location (0.0 0.0 200.0))) (`self.SaveGameReference`)))
  (`GameplayStatics.SaveGameToSlot` (`self.SaveGameReference`) (`self.CheckpontSave`))
  (`KismetSystemLibrary.PrintString` (`KismetStringLibrary.Concat_StrStr` "Save Game" "Trasform" (`KismetStringLibrary.Conv_TransformToString` _output_get))))

(fn `UserConstructionScript`)