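; EnemigoSigue_BP is an enemy that chases the player character (SAM) and calls Empujado (pushed) on it.
; PawnSensing sets a seen flag that is never cleared here and starts an AIMoveTo toward the player.
; When the move succeeds, a debug-drawn PhysicsBody trace runs from the enemy along the X component of its control forward vector.
; Empujado fires only if that trace hits nothing.
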(event `self.PawnSensing.OnSeePawn`
  (params (Pawn :type "Pawn Object Reference"))
  (set `self.EstaViendo aSam?` true)
  (`self.FollowSam`))

(event `FollowSam`
  (bind _returnvalue (`self.K2_GetActorLocation`))
  (if (`self.EstaViendo aSam?`)
    (`|AIMoveTo` self (0.0 0.0 0.0) (`GameplayStatics.GetPlayerCharacter` 0) 0.0
      (:`OnSuccess`
        (bind (_outhit _returnvalue_2) (`KismetSystemLibrary.LineTraceSingleForObjects` :`Start` _returnvalue :`End` (+ _returnvalue (* (`KismetMathLibrary.GetForwardVector` (`self.GetControlRotation`)) (3000.0 0.0 0.0))) :`ObjectTypes` (`|MakeArray` "ObjectTypeQuery4" :!type "EObjectTypeQuery Enum") :`DrawDebugType` "ForDuration"))
        (if (not _returnvalue_2)
          (bind _assam (cast `/Game/Come_Back/Mi_Personaje/SAM` (`GameplayStatics.GetPlayerCharacter` 0)))
          (`/Game/Come_Back/Mi_Personaje/SAM.Empujado` _assam))))))

(fn `UserConstructionScript`)